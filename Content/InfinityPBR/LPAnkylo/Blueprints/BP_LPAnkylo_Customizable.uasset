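; BP_LPAnkylo_Customizable is a low-poly Ankylosaurus actor with optional spike and horn parts that can be toggled per instance.
; The construction script makes the nude body mesh the master pose component for the chin, front leg, back leg and back spike meshes and the head horns, so they follow its animation.
; Boolean variables then set each part's visibility; the event graph has no active logic.
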(event EventBeginPlay)

(event Collision|EventActorBeginOverlap
  (params (OtherActor :type Actor%20Object%20Reference)))

(event EventTick
  (params (DeltaSeconds :type Float%20%28single-precision%29)))

(fn ConstructionScript
  (Class|SkinnedMeshComponent|SetMasterPoseComponent (Variables|Default|GetSK_LPAnkylo_ChinSpikes) (Variables|Default|GetSK_LPAnkylo_Nude) true)
  (Utilities|FlowControl|Sequence
    (:then_0
      (Rendering|SetVisibility (Variables|Default|GetSK_LPAnkylo_BackLegsSpikes) (Variables|Default|GetShowBackLegSpikes) false))
    (:then_1
      (Rendering|SetVisibility (Variables|Default|GetSK_LPAnkylo_ChinSpikes) (Variables|Default|GetShowChinSpikes) false))
    (:then_2
      (Rendering|SetVisibility (Variables|Default|GetSK_LPAnkylo_FrontLegsSpikes) (Variables|Default|GetShowFrontLegSpikes) false))
    (:then_3
      (Rendering|SetVisibility (Variables|Default|GetSK_LPAnkylo_HeadHorns) (Variables|Default|GetShowHeadHorns) false))
    (:then_4
      (Rendering|SetVisibility (Variables|Default|GetSK_LPAnkylo_BackSpikes) (Variables|Default|GetShowBackSpikes) false))))
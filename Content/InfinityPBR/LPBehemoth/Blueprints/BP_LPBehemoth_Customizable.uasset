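; Customizable low-poly Behemoth creature actor, assembled from modular skeletal mesh parts with optional horn, teeth, and head, shoulder and wrist spikes.
; The construction script makes the nude body mesh the master pose component for every accessory, so all parts follow its skeleton.
; It then sets each part's visibility from its own boolean, with separate left and right toggles for shoulder and wrist spikes.
; The event graph holds no active logic.
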(event EventBeginPlay)

(event Collision|EventActorBeginOverlap
  (params (OtherActor :type Actor%20Object%20Reference)))

(event EventTick
  (params (DeltaSeconds :type Float%20%28single-precision%29)))

(fn ConstructionScript
  (Class|SkinnedMeshComponent|SetMasterPoseComponent (Variables|Default|GetSK_LPBehemoth_Horn) (Variables|Default|GetSK_LPBehemoth_Nude) true)
  (Utilities|FlowControl|Sequence
    (:then_0
      (Rendering|SetVisibility (Variables|Default|GetSK_LPBehemoth_HeadSpikes) (Variables|Default|GetShowHeadSpikes) false))
    (:then_1
      (Rendering|SetVisibility (Variables|Default|GetSK_LPBehemoth_Horn) (Variables|Default|GetShowHorn) false))
    (:then_2
      (Rendering|SetVisibility (Variables|Default|GetSK_LPBehemoth_ShoulderSpikesL) (Variables|Default|GetShowLeftShoulderSpikes) false))
    (:then_3
      (Rendering|SetVisibility (Variables|Default|GetSK_LPBehemoth_ShoulderSpikesR) (Variables|Default|GetShowRightShoulderSpikes) false))
    (:then_4
      (Rendering|SetVisibility (Variables|Default|GetSK_LPBehemoth_Teeth) (Variables|Default|GetShowTeeth) false))
    (:then_5
      (Rendering|SetVisibility (Variables|Default|GetSK_LPBehemoth_WristSpikesL) (Variables|Default|GetShowLeftWristSpikes) false))
    (:then_6
      (Rendering|SetVisibility (Variables|Default|GetSK_LPBehemoth_WristSpikesR) (Variables|Default|GetShowRightWristSpikes) false))))
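; Customizable modular Bomber Bug creature Blueprint with optional carapace, wings, pincers and horns.
; The construction script makes the body mesh the master pose component for the four part meshes, so they follow its pose.
; It then sets each part's visibility from its own Show variable.
; The event graph holds only disabled placeholder events, so the Blueprint adds no runtime logic.
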(event EventBeginPlay)

(event Collision|EventActorBeginOverlap
  (params (OtherActor :type Actor%20Object%20Reference)))

(event EventTick
  (params (DeltaSeconds :type Float%20%28single-precision%29)))

(fn ConstructionScript
  (Class|SkinnedMeshComponent|SetMasterPoseComponent (Variables|Default|GetSK_LPBomberBug_Wings) (Variables|Default|GetSK_LPBomberBug_Body) false)
  (Utilities|FlowControl|Sequence
    (:then_0
      (Rendering|SetVisibility (Variables|Default|GetSK_LPBomberBug_Carapace) (Variables|Default|GetShowCarapace) false))
    (:then_1
      (Rendering|SetVisibility (Variables|Default|GetSK_LPBomberBug_Wings) (Variables|Default|GetShowWings) false))
    (:then_2
      (Rendering|SetVisibility (Variables|Default|GetSK_LPBomberBug_Pincers) (Variables|Default|GetShowPincers) false))
    (:then_3
      (Rendering|SetVisibility (Variables|Default|GetSK_LPBomberBug_Horns) (Variables|Default|GetShowHorns) false))))
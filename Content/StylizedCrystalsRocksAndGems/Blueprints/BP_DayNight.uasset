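; BP_DayNight switches a level between day and night lighting based on the IsDay flag.
; Its construction script sets the referenced directional light's intensity and rotation, plus the height fog's directional inscattering colour and volumetric emissive, from day or night variables.
; The SwitchLight event is empty; a similar toggle branch that flips IsDay and omits fog emissive sits unconnected, so switching happens only on construction.
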(event Custom|SwitchLight)

(fn ConstructionScript
  (if (Variables|Default|GetbIsDay?)
    (Utilities|FlowControl|Sequence
      (:then_0
        (Rendering|Components|Light|SetIntensity (Variables|/Script/Engine.Light|GetLightComponent (Variables|Default|GetDirectionalLight)) (Variables|Default|GetLightIntensity_Day)))
      (:then_1
        (Transformation|SetActorRotation (Variables|Default|GetDirectionalLight) (Variables|Default|GetLightPosition_Day)))
      (:then_2
        (Class|ExponentialHeightFogComponent|SetDirectionalInscatteringColor (Variables|/Script/Engine.ExponentialHeightFog|GetComponent (Variables|Default|GetExponentialHeightFog)) (Variables|Default|GetFogColour_Day)))
      (:then_3
        (Class|ExponentialHeightFogComponent|SetVolumetricFogEmissive (Variables|/Script/Engine.ExponentialHeightFog|GetComponent (Variables|Default|GetExponentialHeightFog)) (Variables|Default|GetFogEmissive_Day)))
      (:then_4
        (Variables|Default|SetbIsDay? true)))
    (else
      (Utilities|FlowControl|Sequence
        (:then_0
          (Rendering|Components|Light|SetIntensity (Variables|/Script/Engine.Light|GetLightComponent (Variables|Default|GetDirectionalLight)) (Variables|Default|GetLightIntensity_Night)))
        (:then_1
          (Transformation|SetActorRotation (Variables|Default|GetDirectionalLight) (Variables|Default|GetLightPosition_Night)))
        (:then_2
          (Class|ExponentialHeightFogComponent|SetDirectionalInscatteringColor (Variables|/Script/Engine.ExponentialHeightFog|GetComponent (Variables|Default|GetExponentialHeightFog)) (Variables|Default|GetFogColour_Night)))
        (:then_3
          (Class|ExponentialHeightFogComponent|SetVolumetricFogEmissive (Variables|/Script/Engine.ExponentialHeightFog|GetComponent (Variables|Default|GetExponentialHeightFog)) (Variables|Default|GetFogEmissive_Night)))
        (:then_4
          (Variables|Default|SetbIsDay? false))))))
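; Demo hovercraft pawn that the hero boards through interaction, pilots, and exits.
; HoverControllerBP handles movement, look, jump, rotation, free camera and hovering while unpossessed, while Tick also spins four rotor fans.
; Boarding swaps input mapping to vehicle, disables hero collision, attaches the hero to PlayerSeat, possesses the craft and raises hover height.
; Exiting repossesses and detaches the hero, then lowers hover height.
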(event Custom|OnPosses
  (bind _returnvalue (Game|GetPlayerController 0))
  (bind _herocharacter (Variables|Default|GetHeroCharacter))
  (bind _returnvalue_2 (PlayerController|LocalPlayerSubsystems|GetEnhancedInputLocalPlayerSubsystem _returnvalue))
  (Utilities|IsValid _returnvalue_2
    (:Is%20Valid
      (Input|RemoveMappingContext _returnvalue_2 "/Game/Starwrecked/Input/IM_Hero.IM_Hero" "(bIgnoreAllPressedKeysUntilRelease=True,bForceImmediately=False)")
      (Input|AddMappingContext _returnvalue_2 "/Game/Starwrecked/Input/IM_Vehicle.IM_Vehicle" 0 "(bIgnoreAllPressedKeysUntilRelease=True,bForceImmediately=False)")
      (Utilities|IsValid _herocharacter
        (:Is%20Valid
          (Collision|SetCollisionEnabled (Variables|/Script/Engine.Character|GetCapsuleComponent _herocharacter) "NoCollision")
          (Transformation|AttachComponentToComponent _herocharacter (Variables|Default|GetPlayerSeat) "None" "SnapToTarget" "SnapToTarget" "KeepRelative" false)
          (Game|Player|SetViewTargetwithBlend (Game|GetPlayerController 0) self 3.0 "VTBlend_Linear" 0.0 false))))))

(event Input|EnhancedActionEvents|EnhancedInputActionIA_Jump
  (params (ActionValue :type Boolean) (ElapsedSeconds :type Float%20%28double-precision%29) (TriggeredSeconds :type Float%20%28double-precision%29) (InputAction :type Input%20Action%20Object%20Reference :default "/Game/ThirdPerson/Input/Actions/IA_Jump.IA_Jump"))
  ;[1 1 1] Make Actor Jump
  (:Started
    (Default|Jump (Variables|Default|GetHover_Controller_BP) 1.5e+03 false 0.0)))

(event Input|EnhancedActionEvents|EnhancedInputActionIA_MoveForward
  (params (ActionValue :type Float%20%28double-precision%29) (ElapsedSeconds :type Float%20%28double-precision%29) (TriggeredSeconds :type Float%20%28double-precision%29) (InputAction :type Input%20Action%20Object%20Reference :default "/Game/Starwrecked/Input/IA_MoveForward.IA_MoveForward"))
  ;[1 1 1] Movement Input Events
  (:Triggered
    (Default|AddForwardMovement (Variables|Default|GetHover_Controller_BP) ActionValue)))

(event Input|EnhancedActionEvents|EnhancedInputActionIA_MoveRight
  (params (ActionValue :type Float%20%28double-precision%29) (ElapsedSeconds :type Float%20%28double-precision%29) (TriggeredSeconds :type Float%20%28double-precision%29) (InputAction :type Input%20Action%20Object%20Reference :default "/Game/Starwrecked/Input/IA_MoveRight.IA_MoveRight"))
  ;[1 1 1] Movement Input Events
  (:Triggered
    (Default|AddSidewaysMovement (Variables|Default|GetHover_Controller_BP) ActionValue)))

(event Input|EnhancedActionEvents|EnhancedInputActionIA_TurnRight
  (params (ActionValue :type Float%20%28double-precision%29) (ElapsedSeconds :type Float%20%28double-precision%29) (TriggeredSeconds :type Float%20%28double-precision%29) (InputAction :type Input%20Action%20Object%20Reference :default "/Game/Starwrecked/Input/IA_TurnRight.IA_TurnRight"))
  ;[1 1 1] Movement Input Events
  (:Triggered
    (Default|AddLookatDirection (Variables|Default|GetHover_Controller_BP) ActionValue (stale Input|EnhancedActionEvents|EnhancedInputActionIA_LookUp ActionValue))))

(event Input|EnhancedActionEvents|EnhancedInputActionIA_LookUp
  (params (ActionValue :type Float%20%28double-precision%29) (ElapsedSeconds :type Float%20%28double-precision%29) (TriggeredSeconds :type Float%20%28double-precision%29) (InputAction :type Input%20Action%20Object%20Reference :default "/Game/Starwrecked/Input/IA_LookUp.IA_LookUp"))
  ;[1 1 1] Movement Input Events
  (:Triggered
    (Default|AddLookatDirection (Variables|Default|GetHover_Controller_BP) (stale Input|EnhancedActionEvents|EnhancedInputActionIA_TurnRight ActionValue) ActionValue)))

(event Input|EnhancedActionEvents|EnhancedInputActionIA_RotateVehicleRight
  (params (ActionValue :type Float%20%28double-precision%29) (ElapsedSeconds :type Float%20%28double-precision%29) (TriggeredSeconds :type Float%20%28double-precision%29) (InputAction :type Input%20Action%20Object%20Reference :default "/Game/Starwrecked/Input/IA_RotateVehicleRight.IA_RotateVehicleRight"))
  ;[1 1 1] Movement Input Events
  (:Triggered
    (Default|RotateActorAxisInput (Variables|Default|GetHover_Controller_BP) ActionValue)))

(event Input|EnhancedActionEvents|EnhancedInputActionIA_ExitVehicle
  (params (ActionValue :type Boolean) (ElapsedSeconds :type Float%20%28double-precision%29) (TriggeredSeconds :type Float%20%28double-precision%29) (InputAction :type Input%20Action%20Object%20Reference :default "/Game/Starwrecked/Input/IA_ExitVehicle.IA_ExitVehicle"))
  (bind _returnvalue (Game|GetPlayerController 0))
  (bind _herocharacter (Variables|Default|GetHeroCharacter))
  (:Started
    (Utilities|IsValid (Variables|Default|GetHeroCharacter)
      (:Is%20Valid
        (Game|Player|SetViewTargetwithBlend _returnvalue _herocharacter 0.5 "VTBlend_Linear" 0.0 false)
        (Pawn|Possess _returnvalue _herocharacter)
        (Default|OnPosses _herocharacter)
        (Transformation|DetachFromActor (Variables|Default|GetHeroCharacter) "KeepWorld" "KeepWorld" "KeepRelative")
        (Variables|/Game/Hover_Controller/Blueprints/Hover_Controller_BP.Hover_Controller_BP_C|SetHover%20Height (Variables|Default|GetHover_Controller_BP) 1e+02)))))

(event EventTick
  (params (DeltaSeconds :type Float%20%28single-precision%29))
  ;[1 1 1] Tick Events
  (Utilities|FlowControl|Sequence
    (:then_0
      ;;[1 1 1] Spin Rotors
      (Transformation|AddLocalRotation (Variables|Default|GetHover_Fan4) (Math|Rotator|MakeRotator 0.0 0.0 (* (Utilities|Time|GetWorldDeltaSeconds) (Variables|Default|GetRotation%20Per%20Second) 3.6e+02)) false false))
    (:then_1
      ;;[1 1 1] Keep Actor Hovering While Not Possessed
      (Default|NotPossesedHoverTick (Variables|Default|GetHover_Controller_BP)))))

(event EventOnInteract
  (bind _asbp_hero (Utilities|Casting|CastToBP_Hero (Pawn|GetControlledPawn (Game|GetPlayerController 0))))
  (Variables|Default|SetHeroCharacter _asbp_hero)
  (CallFunction|OnPosses)
  (Variables|/Game/Hover_Controller/Blueprints/Hover_Controller_BP.Hover_Controller_BP_C|SetHover%20Height (Variables|Default|GetHover_Controller_BP) 4e+02)
  (Pawn|Possess (Game|GetPlayerController 0) self))

(event Input|MouseEvents|RightMouseButton
  (params (Key :type Key%20Structure :default "None"))
  (bind _hover_controller_bp (Variables|Default|GetHover_Controller_BP))
  ;[1 1 1] Control Free Camera Rotaiton
  (:Pressed
    (Default|FreeCameraRotation _hover_controller_bp false))
  (:Released
    (Default|FreeCameraRotation _hover_controller_bp true)))

(fn ConstructionScript)